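; BP_BoxActor is a box actor that travels along the spline of a referenced spline actor.
; On BeginPlay it casts the game mode to BP_ThirdPersonGameMode and sets a timeline's play rate to the inverse of SpeedOfBlocks, so that value acts as a travel duration.
; Each timeline update maps the track alpha to a distance along the spline and applies that point's world location and rotation to the actor.
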(event Custom|set%20movement
  (bind _splineref (Variables|Default|GetsplineREF))
  (bind _spline (Variables|/Game/blueprints/BP_SplineActor.BP_SplineActor_C|GetSpline _splineref))
  (Utilities|Casting|CastToBP_ThirdPersonGameMode (Game|GetGameMode))
  (Components|Timeline|SetPlayRate (Variables|Default|GetTarget) (/ 1.0 (Variables|Default|GetSpeed%20Of%20Blocks)))
  (bind _newtrack_0 (Timeline|Timeline Play)
    (:Update
      (Transformation|SetActorLocationAndRotation (Spline|GetLocationatDistanceAlongSpline _spline (Math|Float|Lerp 0.0 (Spline|GetSplineLength _spline) _newtrack_0) "World") (Spline|GetRotationatDistanceAlongSpline _spline (Math|Float|Lerp 0.0 (Spline|GetSplineLength _spline) _newtrack_0) "World")))))

(event EventBeginPlay
  (CallFunction|SetMovement))

(event EventTick
  (params (DeltaSeconds :type Float%20%28single-precision%29)))

(fn ConstructionScript)